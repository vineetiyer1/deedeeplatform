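; Player controller for the 2D PaperZD archer that handles horizontal movement, jumping, dashing and bow shooting through Enhanced Input.
; Holding shoot locks movement and, past a threshold, flags a higher-damage special shot; release spawns an arrow at the pawn interface's spawn point.
; Dash uses a timeline-driven swept offset along facing, followed by a cooldown.
; Tick moves the camera spring arm at fixed height and sets facing from X velocity.
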(event Input|EnhancedActionEvents|EnhancedInputActionIA_Jump
  (params (ActionValue :type Boolean) (ElapsedSeconds :type Float%20%28double-precision%29) (TriggeredSeconds :type Float%20%28double-precision%29) (InputAction :type Input%20Action%20Object%20Reference :default "/Game/2D/Inputs/IA_Jump.IA_Jump"))
  (bind _2dcharacter (Variables|Default|Get2DCharacter))
  (:Started
    (if (not (Variables|Default|GetCharacterMovementLock))
      (Utilities|IsValid _2dcharacter
        (:Is%20Valid
          (Character|Jump _2dcharacter)))))
  (:Completed
    (Utilities|IsValid _2dcharacter
      (:Is%20Valid
        (Character|StopJumping _2dcharacter)))))

(event Input|EnhancedActionEvents|EnhancedInputActionIA_Move
  (params (ActionValue :type Vector%202D%20Structure) (ElapsedSeconds :type Float%20%28double-precision%29) (TriggeredSeconds :type Float%20%28double-precision%29) (InputAction :type Input%20Action%20Object%20Reference :default "/Game/2D/Inputs/IA_Move.IA_Move"))
  (bind _pawnref (Variables|Default|GetPawnRef))
  (:Triggered
    (Utilities|IsValid _pawnref
      (:Is%20Valid
        (if (not (Variables|Default|GetCharacterMovementLock))
          (Pawn|Input|AddMovementInput _pawnref "1.000000,0.000000,0.000000" (.x ActionValue) false))))))

(event Input|EnhancedActionEvents|EnhancedInputActionIA_ShootBow
  (params (ActionValue :type Boolean) (ElapsedSeconds :type Float%20%28double-precision%29) (TriggeredSeconds :type Float%20%28double-precision%29) (InputAction :type Input%20Action%20Object%20Reference :default "/Game/2D/Inputs/IA_ShootBow.IA_ShootBow"))
  (:Triggered
    (Utilities|IsValid (Variables|Default|Get2DCharacter)
      (:Is%20Valid
        (Variables|Default|SetCharacterMovementLock true)
        (CallFunction|DrawBow)
        (if (>= ElapsedSeconds (Variables|Default|GetPowerDrawThreshold))
          (Variables|Default|SetShootSpecialArrow true)
          ;[1 1 1] add effect for special arrow
          (Development|PrintString "Special" true true "(R=0.000000,G=0.660000,B=1.000000,A=1.000000)" 0.0)))))
  (:Completed
    (Utilities|IsValid (Variables|Default|Get2DCharacter)
      (:Is%20Valid
        (if (>= TriggeredSeconds (Variables|Default|GetTimeBeforeNextInput))
          _
          (else
            (Utilities|FlowControl|Delay (- (Variables|Default|GetTimeBeforeNextInput) TriggeredSeconds))))
        (CallFunction|SetArrowDamage (Variables|Default|GetShootSpecialArrow))
        (CallFunction|ShootArrow false)
        (Variables|Default|SetCharacterMovementLock false)
        (Variables|Default|SetisDrawing? false)
        (Variables|Default|SetShootSpecialArrow false)))))

(event Input|EnhancedActionEvents|EnhancedInputActionIA_Dash
  (params (ActionValue :type Boolean) (ElapsedSeconds :type Float%20%28double-precision%29) (TriggeredSeconds :type Float%20%28double-precision%29) (InputAction :type Input%20Action%20Object%20Reference :default "/Game/2D/Inputs/IA_Dash.IA_Dash"))
  (bind _2dcharacter (Variables|Default|Get2DCharacter))
  (bind _returnvalue (Transformation|GetActorLocation _2dcharacter))
  (:Started
    (if (not (Variables|Default|GetDashingLock))
      (Variables|Default|SetDashingLock true)
      (Variables|Default|SetDashing? true)
      (Variables|Default|SetCharacterMovementLock true)
      (CallFunction|SetDashDirection)
      (bind _dashdisplacement (Timeline|DashDistance PlayFromStart)
        (:Update
          (Utilities|IsValid _2dcharacter
            (:Is%20Valid
              (Transformation|SetActorLocation _2dcharacter (Math|Vector|MakeVector (+ (.x _returnvalue) (* (Variables|Default|GetDashBoost) _dashdisplacement)) (.y _returnvalue) (.z _returnvalue)) true false))))
        (:Finished
          (Variables|Default|SetDashing? false)
          (Variables|Default|SetCharacterMovementLock false)
          (Utilities|FlowControl|Delay (Variables|Default|GetPostDashMovementLock))
          (Variables|Default|SetDashingLock false))))))

(event EventBeginPlay
  (bind _self self)
  (bind _returnvalue (PlayerController|LocalPlayerSubsystems|GetEnhancedInputLocalPlayerSubsystem _self))
  (Utilities|IsValid _returnvalue
    (:Is%20Valid
      (Input|AddMappingContext _returnvalue "/Game/2D/Inputs/IMC_Locomotion.IMC_Locomotion" 0 "(bIgnoreAllPressedKeysUntilRelease=True,bForceImmediately=False)"))))

(event EventTick
  (params (DeltaSeconds :type Float%20%28single-precision%29))
  (bind _2dcharacter (Variables|Default|Get2DCharacter))
  (Utilities|IsValid _2dcharacter
    (:Is%20Valid
      (CallFunction|SetPlayerCameraMovement _2dcharacter)
      (CallFunction|SetCharacterRotationtoControlDirection _2dcharacter))
    (:Is%20Not%20Valid
      (Development|PrintString "Character controller - Player is missing" true true "(R=0.000000,G=0.660000,B=1.000000,A=1.000000)" 0.0))))

(event EventPossess
  (params (PossessedPawn :type Pawn%20Object%20Reference))
  (bind _output_get (Variables|Default|SetPawnRef PossessedPawn))
  (bind _aspaper_zdcharacter (Utilities|Casting|CastToPaperZDCharacter _output_get))
  (bind _output_get_2 (Variables|Default|Set2DCharacter _aspaper_zdcharacter))
  (bind _asbpi_character_components (Utilities|Casting|CastToBPI_CharacterComponents _output_get_2))
  (Variables|Default|SetComponentInterfaceRef _asbpi_character_components))

(fn ConstructionScript)

(fn DrawBow
  (Variables|Default|SetisDrawing? true))

(fn ShootArrow
  (params (Special? :type Boolean))
  (bind _2dcharacter (Variables|Default|Get2DCharacter))
  (Utilities|IsValid (Variables|Default|Get2DCharacter)
    (:Is%20Valid
      (bind (_spawnlocation _spawnrotation) (Default|GetProjectileSpawnLocation (Variables|Default|GetComponentInterfaceRef)))
      (Utilities|IsValid _2dcharacter
        (:Is%20Valid
          (Game|SpawnActorfromClass "/Game/2D/Blueprints/PlayerBP/2D_Characters/PixelAdventurerAnims/ArcherAdventurer/BP_ArrowProjectile.BP_ArrowProjectile_C" (Math|Transform|MakeTransform _spawnlocation (Math|Rotator|MakeRotator (.roll _spawnrotation) (- (.pitch _spawnrotation) 9e+01) (.yaw _spawnrotation)) "1.000000,1.000000,1.000000") "Undefined" "MultiplyWithRoot" 0 _2dcharacter)
          (return))))))

(fn SetArrowDamage
  (params (isSpecial? :type Boolean))
  (if isSpecial?
    (Variables|Default|SetArrowDamage 6e+01)
    (else
      (Variables|Default|SetArrowDamage 3e+01))))

(fn SetPlayerCameraMovement
  (params (Character :type Actor%20Object%20Reference))
  (bind _returnvalue (Transformation|GetActorLocation Character))
  (bind _followarm (Default|GetPlayerCameraSpringArm (Variables|Default|GetComponentInterfaceRef)))
  (Transformation|SetWorldLocation _followarm (Math|Vector|MakeVector (.x _returnvalue) (.y _returnvalue) 7e+01) false false))

(fn SetCharacterRotationtoControlDirection
  (params (CharacterRef :type Character%20Object%20Reference))
  (bind _self self)
  (bind _self_2 self)
  (Math|Float|CompareFloat (.X (Math|Vector|BreakVector (Variables|/Script/Engine.MovementComponent|GetVelocity (Variables|/Script/Engine.Character|GetCharacterMovement CharacterRef)))) 0.0
    (:>
      ;[0 0.4745 1] Look Right
      (Utilities|IsValid _self
        (:Is%20Valid
          (Pawn|SetControlRotation _self (Math|Rotator|MakeRotator 0.0 0.0 0.0)))))
    (:<
      ;[0 0.4745 1] Look Left
      (Utilities|IsValid _self_2
        (:Is%20Valid
          (Pawn|SetControlRotation _self_2 (Math|Rotator|MakeRotator 0.0 0.0 1.8e+02)))))))

(fn SetDashDirection
  (bind _2dcharacter (Variables|Default|Get2DCharacter))
  (Utilities|IsValid _2dcharacter
    (:Is%20Valid
      (bind _output_get (Variables|Default|SetDashBoost (* (Variables|Default|GetDashBoostMultiplier) (.x (Transformation|GetActorForwardVector _2dcharacter)))))
      (return _output_get))))

(fn GetArrowDamage
  (return (Variables|Default|GetArrowDamage)))

(fn GetDashing
  (return (Variables|Default|GetDashing?)))

(fn GetHealth
  (return 0.0))

(fn GetIsDrawingforArcher
  (return (Variables|Default|GetisDrawing?)))

(fn GetIsEnemyHit
  (return false))

(fn GetTimeBeforeNextInput
  (return (Variables|Default|GetTimeBeforeNextInput)))