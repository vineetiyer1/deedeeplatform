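; BP_HollowArcher is a Blueprint for an archer character among the 2D pixel adventurer player characters.
; It holds almost no logic: its event nodes are disabled and its construction script only calls the parent.
; Two getters expose its components, returning the FollowArm as the camera spring arm and the ProjectileSpawn world location and rotation as the projectile spawn point.
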(event EventBeginPlay
  (|CallParentFunction) ; This node is disabled and will not be called.\nDrag off pins to build functionality.
)

(event Collision|EventActorBeginOverlap
  (params (OtherActor :type Actor%20Object%20Reference))
  (|CallParentFunction OtherActor) ; This node is disabled and will not be called.\nDrag off pins to build functionality.
)

(event EventTick
  (params (DeltaSeconds :type Float%20%28single-precision%29))
  (|CallParentFunction DeltaSeconds) ; This node is disabled and will not be called.\nDrag off pins to build functionality.
)

(fn ConstructionScript
  (|CallParentFunction))

(fn GetPlayerCameraSpringArm
  (return (Variables|Default|GetFollowArm)))

(fn GetProjectileSpawnLocation
  (bind _projectilespawn (Variables|Default|GetProjectileSpawn))
  (bind _returnvalue (Transformation|GetWorldTransform _projectilespawn))
  (return (.location _returnvalue) (.rotation _returnvalue)))