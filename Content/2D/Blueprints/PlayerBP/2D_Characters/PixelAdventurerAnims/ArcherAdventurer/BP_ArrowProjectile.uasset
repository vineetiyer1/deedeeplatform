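; BP_ArrowProjectile is the arrow fired by the 2D pixel archer adventurer, damaging what it hits.
; On BeginPlay it caches the player controller's combat status interface.
; On collision overlap it ignores itself, other arrows and its instigator, then applies damage read live through that interface and destroys itself.
; Damage is always credited to player controller 0, and each hit prints a debug message.
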(event OnComponentBeginOverlap(Collision)
  (params (OverlappedComponent :type Primitive%20Component%20Object%20Reference) (OtherActor :type Actor%20Object%20Reference) (OtherComp :type Primitive%20Component%20Object%20Reference) (OtherBodyIndex :type Integer) (bFromSweep :type Boolean) (SweepResult :type Hit%20Result%20Structure%20%28by%20ref%29))
  (if (Math|Boolean|ANDBoolean (!= OtherActor self) (not (Class|GameplayStatics|ObjectIsA OtherActor (Utilities|GetClass self))) (!= OtherActor (Game|GetInstigator)))
    (Development|PrintString (Utilities|String|Append "Hit Actor: " (Utilities|GetDisplayName OtherActor)) true true "(R=0.000000,G=0.660000,B=1.000000,A=1.000000)" 1.0)
    (bind _damage (Default|GetArrowDamage (Variables|Default|GetCombatStatusInterfaceRef)))
    (Game|Damage|ApplyDamage OtherActor _damage (Game|GetPlayerController 0) self "/Script/Engine.DamageType")
    (Actor|DestroyActor)))

(event EventBeginPlay
  (bind _asbpi_character_combat_status (Utilities|Casting|CastToBPI_CharacterCombatStatus (Game|GetPlayerController 0)))
  (Variables|Default|SetCombatStatusInterfaceRef _asbpi_character_combat_status))

(event EventTick
  (params (DeltaSeconds :type Float%20%28single-precision%29)))

(fn ConstructionScript)