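; BP_MushroomMan is a 2D mushroom enemy that takes damage and exposes its combat status.
; AnyDamage sets IsHit, subtracts Health and prints it.
; While alive, it clears IsHit after a delay read from the player controller's BPI_CharacterCombatStatus interface; at zero Health it disables collision and leaves IsHit set.
; Getters report Health and IsHit, including GetIsDrawingForArcher, which also returns IsHit; its own GetTimeBeforeNextInput is empty.
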(event EventBeginPlay
  (bind _asbpi_character_combat_status (Utilities|Casting|CastToBPI_CharacterCombatStatus (Game|GetPlayerController 0)))
  (Variables|Default|SetAs%20BPI%20Character%20Combat%20Status _asbpi_character_combat_status))

(event Collision|EventActorBeginOverlap
  (params (OtherActor :type Actor%20Object%20Reference)))

(event EventTick
  (params (DeltaSeconds :type Float%20%28single-precision%29)))

(event Game|Damage|EventAnyDamage
  (params (Damage :type Float%20%28single-precision%29) (DamageType :type Damage%20Type%20Object%20Reference) (InstigatedBy :type Controller%20Object%20Reference) (DamageCauser :type Actor%20Object%20Reference))
  (Variables|Default|SetisHit true)
  (CallFunction|TakeDamage Damage)
  (Development|PrintString (Utilities|String|ToString(Float) (Variables|Default|GetHealth)) true true "(R=0.000000,G=0.660000,B=1.000000,A=1.000000)" 1.0)
  (bind _timeoffset (Default|GetTimeBeforeNextInput (Variables|Default|GetAs%20BPI%20Character%20Combat%20Status)))
  (if (> (Variables|Default|GetHealth) 0.0)
    (Utilities|FlowControl|Delay _timeoffset)
    (Variables|Default|SetisHit false)
    (else
      (Collision|SetActorEnableCollision false))))

(fn ConstructionScript)

(fn TakeDamage
  (params (Damage :type Float%20%28double-precision%29))
  (Variables|Default|SetHealth (- (Variables|Default|GetHealth) Damage)))

(fn GetHealth
  (return (Variables|Default|GetHealth)))

(fn GetIsDrawingforArcher
  (return (Variables|Default|GetisHit)))

(fn GetIsEnemyHit
  (return (Variables|Default|GetisHit)))

(fn GetTimeBeforeNextInput)