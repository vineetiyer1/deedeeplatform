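; Game mode for the 2D archer game that makes the background follow the player horizontally.
; On BeginPlay it caches the archer player controller, its PaperZD pawn, the BP_Background actor and that actor's starting Y.
; Each tick it eases the background's X toward the player's X with FInterpTo, keeping the cached Y.
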(event EventBeginPlay
  (bind _returnvalue (Game|GetPlayerController 0))
  (bind _asbpc_archer (Utilities|Casting|CastToBPC_Archer _returnvalue))
  (Variables|Default|SetPCRef _asbpc_archer)
  (bind _aspaper_zdcharacter (Utilities|Casting|CastToPaperZDCharacter (Pawn|GetControlledPawn _returnvalue)))
  (Variables|Default|SetPlayerCharacterRef _aspaper_zdcharacter)
  (bind _returnvalue_2 (Actor|GetActorOfClass "/Game/2D/Blueprints/GameElements/BackgroundActors/BP_Background.BP_Background_C"))
  (Variables|Default|SetBackground _returnvalue_2)
  (Utilities|IsValid (Variables|Default|GetBackground)
    (:Is%20Valid
      (Variables|Default|SetBackgroundYPosition (.y (Transformation|GetActorLocation (Variables|Default|GetBackground)))))))

(event EventTick
  (params (DeltaSeconds :type Float%20%28single-precision%29))
  (bind _background (Variables|Default|GetBackground))
  (bind _playercharacterref (Variables|Default|GetPlayerCharacterRef))
  (Utilities|IsValid _playercharacterref
    (:Is%20Valid
      (Transformation|SetActorLocation _background (Math|Vector|MakeVector (Math|Interpolation|FInterpTo (.x (Transformation|GetActorLocation _background)) (.x (Transformation|GetActorLocation _playercharacterref)) DeltaSeconds 1e+01) (Variables|Default|GetBackgroundYPosition) 0.0) false false))))

(fn ConstructionScript)