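; BP_TM_Collapsible is a 2D Paper2D tile map element that collapses temporarily when hit, then reappears.
; The Hit event plays CollapseTimeline, whose Flicker track is added to the tile map's current relative X each update.
; When the timeline finishes, the tile map is hidden with collision disabled, then restored to visible and solid after a Duration delay.
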(event EventBeginPlay)

(event Collision|EventActorBeginOverlap
  (params (OtherActor :type Actor%20Object%20Reference)))

(event Collision|EventHit
  (params (MyComp :type Primitive%20Component%20Object%20Reference) (Other :type Actor%20Object%20Reference) (OtherComp :type Primitive%20Component%20Object%20Reference) (bSelfMoved :type Boolean) (HitLocation :type Vector :default "0, 0, 0") (HitNormal :type Vector :default "0, 0, 0") (NormalImpulse :type Vector :default "0, 0, 0") (Hit :type Hit%20Result%20Structure%20%28by%20ref%29))
  (bind _papertilemap (Variables|Default|GetPaperTileMap))
  (bind _papertilemap_2 (Variables|Default|GetPaperTileMap))
  (bind _relativelocation (Variables|/Script/Engine.SceneComponent|GetRelativeLocation _papertilemap))
  (bind _flicker (Timeline|CollapseTimeline PlayFromStart)
    (:Update
      (Transformation|SetRelativeTransform _papertilemap (Math|Transform|MakeTransform (Math|Vector|MakeVector (+ (.x _relativelocation) _flicker) (.y _relativelocation) (.z _relativelocation)) "0, 0, 0" "1.000000,1.000000,1.000000") false false))
    (:Finished
      (Rendering|SetVisibility _papertilemap_2 false false)
      (Collision|SetCollisionEnabled _papertilemap_2 "NoCollision")
      (Utilities|FlowControl|Delay (Variables|Default|GetDuration))
      (Collision|SetCollisionEnabled _papertilemap_2 "QueryAndPhysics")
      (Rendering|SetVisibility _papertilemap_2 true false))))

(fn ConstructionScript)